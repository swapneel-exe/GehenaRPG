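; BP_Item is an item actor that shows an equip prompt while the RPG character overlaps it.
; Begin overlap sets IsOverlappingItems on the character, creates an EquipItemPrompt widget, passes it to SetCorrectItemName and adds it to the viewport.
; End overlap clears the flag and removes every top-level EquipItemPrompt widget.
; SetCorrectItemName is empty here, so this Blueprint leaves the prompt's item name unset.
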(event EventBeginPlay)

(event Collision|EventActorBeginOverlap
  (params (OtherActor :type Actor%20Object%20Reference))
  (bind _asrpgcharacter (Utilities|Casting|CastToRPGCharacter OtherActor))
  (Variables|/Script/RPG.RPGCharacter|SetisOverlappingItems _asrpgcharacter true)
  (bind _returnvalue (UserInterface|CreateWidget "/Game/UIWidgets/EquipItemPrompt.EquipItemPrompt_C"))
  (CallFunction|SetCorrectItemName _returnvalue)
  (UserInterface|Viewport|AddtoViewport _returnvalue 0))

(event EventTick
  (params (DeltaSeconds :type Float%20%28single-precision%29)))

(event Collision|EventActorEndOverlap
  (params (OtherActor :type Actor%20Object%20Reference))
  (bind _asrpgcharacter (Utilities|Casting|CastToRPGCharacter OtherActor))
  (Variables|/Script/RPG.RPGCharacter|SetisOverlappingItems _asrpgcharacter false)
  (bind _foundwidgets (Widget|GetAllWidgetsOfClass "/Game/UIWidgets/EquipItemPrompt.EquipItemPrompt_C" true))
  (for _array_element _foundwidgets
    (Widget|RemovefromParent _array_element)))

(fn ConstructionScript)

(fn SetCorrectItemName
  (params (WidgetReference :type Equip%20Item%20Prompt%20Object%20Reference)))